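; BP_MissionAreaVolume is a volume that tracks whether BP_Marine2 is inside the mission area.
; Begin and end overlap toggle the marine's OutsideMissionArea flag, clearing a timer on entry and setting one for SecondsBeforePlayerDeath on exit.
; Neither timer node names a function, so nothing shown calls KillPlayer.
; KillPlayer prints a debug string and calls ApplyDamage on the player character with no damage amount set.
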(event EventBeginPlay)

(event Collision|EventActorBeginOverlap
  (params (OtherActor :type Actor%20Object%20Reference))
  (bind _asbp_marine_2 (Utilities|Casting|CastToBP_Marine2 OtherActor))
  (Variables|/Game/Blueprint/Pawns/BP_Marine2.BP_Marine2_C|SetOutside%20Mission%20Area _asbp_marine_2 false)
  (Utilities|Time|ClearTimerbyFunctionName 0 ""))

(event EventTick
  (params (DeltaSeconds :type Float%20%28single-precision%29)))

(event Collision|EventActorEndOverlap
  (params (OtherActor :type Actor%20Object%20Reference))
  (bind _asbp_marine_2 (Utilities|Casting|CastToBP_Marine2 OtherActor))
  (Variables|/Game/Blueprint/Pawns/BP_Marine2.BP_Marine2_C|SetOutside%20Mission%20Area _asbp_marine_2 true)
  (Utilities|Time|SetTimerbyFunctionName 0 "" (Variables|Default|GetSeconds%20Before%20Player%20Death)))

(fn ConstructionScript)

(fn KillPlayer
  (Development|PrintString "Hello")
  (Game|Damage|ApplyDamage (Game|GetPlayerCharacter 0) 0.0 0 0))