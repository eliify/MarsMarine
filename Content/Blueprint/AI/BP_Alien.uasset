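; Alien enemy character that chases the player, attacks in melee and can be killed.
; A self-restarting AIMoveTo loop drives pursuit, while AttackBox overlap with BP_Marine2 runs a looping timer that plays the attack montage when in range, halting movement until completion.
; DamagePlayer applies the hit but is not called within this Blueprint.
; Lethal damage disables collision, credits the player's kill, notifies BP_Marine_Gamemode and destroys the actor after a delay.
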(event OnComponentBeginOverlap(AttackBox)
  (params (OverlappedComponent :type Primitive%20Component%20Object%20Reference) (OtherActor :type Actor%20Object%20Reference) (OtherComp :type Primitive%20Component%20Object%20Reference) (OtherBodyIndex :type Integer) (bFromSweep :type Boolean) (SweepResult :type Hit%20Result%20Structure%20%28by%20ref%29))
  (Utilities|Casting|CastToBP_Marine2 OtherActor)
  (bind _returnvalue (Utilities|Time|SetTimerbyEvent (delegate Custom|Attack) 1.0 true true))
  (Variables|Default|SetAttackTimerHandle _returnvalue))

(event OnComponentEndOverlap(AttackBox)
  (params (OverlappedComponent :type Primitive%20Component%20Object%20Reference) (OtherActor :type Actor%20Object%20Reference) (OtherComp :type Primitive%20Component%20Object%20Reference) (OtherBodyIndex :type Integer))
  (Utilities|Casting|CastToBP_Marine2 OtherActor)
  (Utilities|Time|ClearandInvalidateTimerbyHandle (Variables|Default|GetAttackTimerHandle)))

(event Custom|Attack
  (if (CallFunction|CanAttack)
    (CallFunction|DeactivateAIMovement)
    (Animation|Montage|PlayMontage (Variables|Character|GetMesh) "/Game/Characters/Enemy_Great_Spider/Animations/Alien_Attack.Alien_Attack"
      (:OnCompleted
        (CallFunction|ActivateAIMovement)))))

(event EventBeginPlay
  (if (CallFunction|IsAlive) :!label _label
    (AI|AIMoveTo self "0, 0, 0" (Game|GetPlayerCharacter 0) 5.0 false
      (:OnSuccess
        _)
      (:OnFail
        _))
    (Utilities|FlowControl|Delay 0.02)
    (Development|PrintString "")
    (goto _label)))

(event Game|Damage|EventAnyDamage
  (params (Damage :type Float%20%28single-precision%29) (DamageType :type Damage%20Type%20Object%20Reference) (InstigatedBy :type Controller%20Object%20Reference) (DamageCauser :type Actor%20Object%20Reference))
  (if (CallFunction|IsAlive)
    (bind _output_get (Variables|Default|SetHealth (- (Variables|Default|GetHealth) Damage)))
    (if (<= _output_get 0.0)
      (CallFunction|DecreaseHealth)
      (if true
        (CallFunction|KillAI)
        (Utilities|FlowControl|Delay 3.0)
        (Actor|DestroyActor)))))

(fn ConstructionScript)

(fn IsWithinAttackRange
  (return (< (Transformation|GetDistanceTo (Game|Player|GetPlayerPawn 0)) (Variables|Default|GetAttack%20Range))))

(fn IsAttacking
  (return (Animation|Montage|MontageIsPlaying (Components|SkeletalMesh|GetAnimInstance (Variables|Character|GetMesh)) "/Game/Characters/Enemy_Great_Spider/Animations/Alien_Attack.Alien_Attack")))

(fn DeactivateAIMovement
  (bind _charactermovement (Variables|Character|GetCharacterMovement))
  (Components|Movement|StopMovementImmediately _charactermovement)
  (Components|Activation|Deactivate _charactermovement))

(fn ActivateAIMovement
  (Components|Activation|Activate (Variables|Character|GetCharacterMovement) false))

(fn DamagePlayer
  (if (CallFunction|IsAlive)
    (Game|Damage|ApplyDamage (Game|GetPlayerCharacter 0) (Variables|Default|GetDamage%20Per%20Hit) 0 0)))

(fn DecreaseHealth)

(fn KillAI
  (Variables|Default|SetDead true)
  (CallFunction|DeactivateAIMovement)
  (Collision|SetActorEnableCollision false)
  (bind _asbp_marine_2 (Utilities|Casting|CastToBP_Marine2 (Game|GetPlayerCharacter 0)))
  (Default|IncreaseKills _asbp_marine_2)
  (bind _asbp_marine_gamemode (Utilities|Casting|CastToBP_Marine_Gamemode (Game|GetGameMode)))
  (Default|RegisterAlienDeath _asbp_marine_gamemode self))

(fn IsAlive
  (return (not (Variables|Default|GetDead))))

(fn CanAttack
  (return (Math|Boolean|ANDBoolean (CallFunction|IsWithinAttackRange) (not (CallFunction|IsAttacking)) (CallFunction|IsAlive))))